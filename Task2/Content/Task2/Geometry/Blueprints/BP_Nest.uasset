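; Nest actor that spawns AI-driven turtles when its SpawnTurtle event is called.
; Each spawn plays a sound and briefly pulses the particle system through ParticularSistemLife.
; It creates an AIC_Turtle controller with the nest's TargetPoint and BehaviorTurtle, spawns a BP_Turtle at SpawnPoint, then has the controller manually possess it.
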(event Custom|SpawnTurtle
  (Audio|PlaySound2D (Variables|Default|GetSoundSpawn) 1.0 1.0 0.0 0 0)
  (CallFunction|ParticularSistemLife)
  (bind _returnvalue (Game|SpawnActorfromClass "/Game/Task2/Characters/Turtle/AIC_Turtle.AIC_Turtle_C" (Math|Transform|MakeTransform "0, 0, 0" "0, 0, 0" "1,1,1") "AlwaysSpawn" 0 (Variables|Default|GetTargetPoint) (Variables|Default|GetBehaviorTurtle) 0))
  (bind _returnvalue_2 (Game|SpawnActorfromClass "/Game/Task2/Characters/Turtle/BP_Turtle.BP_Turtle_C" (Transformation|GetWorldTransform (Variables|Default|GetSpawnPoint)) "AlwaysSpawn" 0 0 0 0))
  (Pawn|Possess _returnvalue _returnvalue_2))

(event Custom|ParticularSistemLife
  (bind _particlesystem (Variables|Default|GetParticleSystem))
  (Components|Activation|Activate _particlesystem false)
  (Utilities|FlowControl|Delay 0.2)
  (Components|Activation|Deactivate _particlesystem))

(fn ConstructionScript)