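; BP_Button is a clickable in-world button that tells a linked Nest to spawn a turtle.
; The construction script shows its Number on a text render, applies the button material and stores the button's initial relative position.
; When a valid Nest is set, clicking spawns the turtle, moves the button to its local origin and swaps the text material; releasing restores both position and material.
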(event OnClicked(Button)
  (params (TouchedComponent :type Primitive%20Component%20Object%20Reference) (ButtonPressed :type Key%20Structure))
  (bind _nest (Variables|Connection|GetNest))
  (Utilities|IsValid _nest
    (:Is%20Valid
      (Default|SpawnTurtle _nest)
      (Transformation|SetRelativeLocation (Variables|Components|GetButton) "0, 0, 0" false false)
      (Class|TextRenderComponent|SetTextMaterial (Variables|Components|GetTextRender) (Variables|Appearance|GetClickedFontMaterial)))))

(event OnReleased(Button)
  (params (TouchedComponent :type Primitive%20Component%20Object%20Reference) (ButtonReleased :type Key%20Structure))
  (Utilities|IsValid (Variables|Connection|GetNest)
    (:Is%20Valid
      (Transformation|SetRelativeLocation (Variables|Components|GetButton) (Variables|Appearance|GetInitialRelativeLocationButton) false false)
      (Class|TextRenderComponent|SetTextMaterial (Variables|Components|GetTextRender) (Variables|Appearance|GetReleasedFontMaterial)))))

(fn ConstructionScript
  (Rendering|Components|TextRender|SetText (Variables|Components|GetTextRender) (Utilities|Text|ToText(Integer) (Variables|Appearance|GetNumber)))
  (Rendering|Material|SetMaterial (Variables|Components|GetButton) 0 (Variables|Appearance|GetButtonMaterial))
  (Variables|Appearance|SetInitialRelativeLocationButton (Variables|/Script/Engine.SceneComponent|GetRelativeLocation (Variables|Components|GetButton))))